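; Inventory component that holds collected items such as keys and owns their on-screen widget, WBP_InventoryUI, shown only while items are held.
; Adding appends to both Items and Collectibles, while consuming matches by CollectablePDA and removes only from Items; both operations fire OnInventoryChanged.
; SaveInstance and LoadInstance copy both arrays to and from save data.
; UpdateVisibilityInventoryUI creates a new widget on each call, at BeginPlay and on load.
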(event `self.ReceiveBeginPlay`
  (`self.UpdateVisibilityInventoryUI`))

(event `UpdateVisibilityInventoryUI`
  (bind _returnvalue (`KismetArrayLibrary.Array_IsEmpty` (`self.Items`)))
  (bind _inventoryui (`self.CreateInventoryUI`))
  (bind _output_get (set `self.Inventory UI` _inventoryui))
  (`KismetSystemLibrary.PrintString` (`KismetStringLibrary.Conv_BoolToString` _returnvalue))
  (if _returnvalue
    (`Widget.SetVisibility` _output_get "Hidden")
    (else
      (`Widget.SetVisibility` _output_get "Visible"))))

(fn `AddCollectable`
  (params (Collectable :type "/Game/Migrated/STR_Collectable Structure"))
  (returns (Success :type Boolean))
  (`KismetArrayLibrary.Array_Add` (`self.Items`) Collectable)
  (`KismetSystemLibrary.PrintString` "Key added in inventory" true true (struct :`R` 1.0 :`B` 0.070606 :`A` 1.0))
  (`KismetArrayLibrary.Array_Add` (`self.Collectibles`) Collectable)
  (`Widget.SetVisibility` (`self.Inventory UI`) "Visible")
  (`self.OnInventoryChanged`)
  (return true))

(fn `ConsumeCollectable`
  (params (Collectable :type "/Game/Migrated/STR_Collectable Structure"))
  (returns (Success :type Boolean))
  (for (_array_element _array_index) (`self.Items`)
    (if (== (`.CollectablePDA_4_B960388147772F1B45C61EACB148C8E7` (break `/Game/Migrated/STR_Collectable` _array_element)) (`.CollectablePDA_4_B960388147772F1B45C61EACB148C8E7` (break `/Game/Migrated/STR_Collectable` Collectable)))
      (break)))
  (`KismetArrayLibrary.Array_Remove` (`self.Items`) _array_index)
  (if (`KismetArrayLibrary.Array_IsEmpty` (`self.Items`))
    (`Widget.SetVisibility` (`self.Inventory UI`) "Hidden"))
  (`self.OnInventoryChanged`)
  (return true))

(fn `CreateInventoryUI`
  (returns (InventoryUI :type "/Game/Assets/Characters/Player/Inventory/UI/WBP_InventoryUI Object Reference"))
  (bind _returnvalue (`|CreateWidget` "/Game/Assets/Characters/Player/Inventory/UI/WBP_InventoryUI.WBP_InventoryUI_C" (`GameplayStatics.GetPlayerController` 0) self))
  (`UserWidget.AddToViewport` _returnvalue 0)
  (return _returnvalue))

(fn `LoadInstance`
  (params (SaveData :type "/SaveSystem/BP_SaveData Object Reference"))
  (returns (Sucess :type Boolean))
  (bind _inventorystruct_items (break `/Game/Migrated/STR_SaveData_Inventory` (`/SaveSystem/BP_SaveData.InventoryStruct` SaveData)))
  (for _array_element _inventorystruct_items
    (`KismetArrayLibrary.Array_Add` (`self.Items`) _array_element))
  (`self.UpdateVisibilityInventoryUI`)
  (`self.OnInventoryChanged`)
  (for _array_element_2 (`/SaveSystem/BP_SaveData.Collectables` SaveData)
    (`KismetArrayLibrary.Array_Add` (`self.Collectibles`) _array_element_2))
  (return true))

(fn `SaveInstance`
  (params (SaveData :type "/SaveSystem/BP_SaveData Object Reference"))
  (returns (Sucess :type Boolean))
  (bind _inventorystruct_items (break `/Game/Migrated/STR_SaveData_Inventory` (`/SaveSystem/BP_SaveData.InventoryStruct` SaveData)))
  (`KismetArrayLibrary.Array_Clear` _inventorystruct_items)
  (for _array_element (`self.Items`)
    (`KismetArrayLibrary.Array_Add` _inventorystruct_items _array_element))
  (for _array_element_2 (`self.Collectibles`)
    (`KismetArrayLibrary.Array_Add` (`/SaveSystem/BP_SaveData.Collectables` SaveData) _array_element_2))
  (return true))