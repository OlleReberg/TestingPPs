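; Time-tracking component that records play time in the save data.
; It stamps the start time on BeginPlay and derives elapsed time by subtracting time-of-day values, leaving the date out.
; SaveInstance adds that elapsed time to the saved TimePlayed and writes it with the current level name and date.
; LoadInstance copies the saved TimePlayed into TotalTime, and the start stamp is not reset on save or load.
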(event `self.ReceiveBeginPlay`
  (set `self.StartTime` (`KismetMathLibrary.Now`)))

(event `self.ReceiveEndPlay`
  (params (EndPlayReason :type "EEndPlayReason Enum" :default "Destroyed")))

(fn `GetElapsedTime`
  (returns (ElapsedTime :type "Timespan Structure"))
  (set `self.StopTime` (`KismetMathLibrary.Now`))
  (return (- (`KismetMathLibrary.GetTimeOfDay` (`self.StopTime`)) (`KismetMathLibrary.GetTimeOfDay` (`self.StartTime`)))))

(fn `LoadInstance`
  (params (SaveData :type "/SaveSystem/BP_SaveData Object Reference"))
  (returns (Sucess :type Boolean))
  (bind (_saveinfo_currentlvl _saveinfo_timeplayed) (break `/Game/Migrated/STR_SaveData_SaveInfo` (`/SaveSystem/BP_SaveData.SaveInfo` SaveData)))
  (set `self.TotalTime` _saveinfo_timeplayed)
  (return true))

(fn `SaveInstance`
  (params (SaveData :type "/SaveSystem/BP_SaveData Object Reference"))
  (returns (Sucess :type Boolean))
  (`self.GetElapsedTime`)
  (bind _returnvalue (`GameplayStatics.GetCurrentLevelName` true))
  (set `/SaveSystem/BP_SaveData.SaveInfo` (make `/Game/Migrated/STR_SaveData_SaveInfo` _returnvalue (+ (struct) (`.TimePlayed_15_26CE57DB478F1DCE5D56D48C87BA7570` (break `/Game/Migrated/STR_SaveData_SaveInfo` (`/SaveSystem/BP_SaveData.SaveInfo` SaveData)))) (`KismetMathLibrary.Now`)) SaveData)
  (return true))