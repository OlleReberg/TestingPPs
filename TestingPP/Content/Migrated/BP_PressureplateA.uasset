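; Pressure plate code puzzle that builds a row of spaced plates, one per character of the correct code.
; The construction script tags each plate with a digit from CodeAssign and binds its overlap event.
; When the first-person character overlaps a plate, its digit joins the input and a tag-indexed plate toggles color.
; At full length it prints the result, then, right or wrong, resets materials and messages interactable objects inside the per-plate loop, clearing input.
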(fn `AddCode`
  (params (Add :type String))
  (bind _inputcode (`self.InputCode`))
  ;[1 1 1] Check if the input code is the same as the correct code
  (set `self.InputCode` (`KismetStringLibrary.Concat_StrStr` _inputcode Add))
  (if (== (`KismetStringLibrary.Len` (`self.CorrectCode`)) (`KismetStringLibrary.Len` _inputcode))
    (if (== (`self.CorrectCode`) (`self.InputCode`))
      (`KismetSystemLibrary.PrintString` "CODE INPUT IS CORRECT!" true true (struct :`G` 1.0 :`B` 0.009438 :`A` 1.0) 10.0)
      (else
        (`KismetSystemLibrary.PrintString` "CODE INCORRECT, TRY AGAIN" true true (struct :`R` 1.0 :`G` 0.013739 :`A` 1.0) 10.0)))
    (for _array_element (`self.Static mesh`)
      (`PrimitiveComponent.SetMaterial` _array_element 0 (`self.PressurePlateBaseMat`))
      (for _array_element_2 (`self.InteractableObject`)
        (message `/Game/Assets/Environment/Interactables/PressurePlates/IF_Interact.Interact` _array_element_2)
        (set `self.InputCode` "")))))

(fn `EventTriggerFunction`
  (params (OverlappedComponent :type "PrimitiveComponent Object Reference") (OtherActor :type "Actor Object Reference") (OtherComp :type "PrimitiveComponent Object Reference") (OtherBodyIndex :type Integer) (bFromSweep :type Boolean) (SweepResult :type "HitResult Structure (by ref)"))
  (bind _returnvalue (`KismetStringLibrary.Conv_NameToString` (`|GetArrayItem` (`ActorComponent.ComponentTags` OverlappedComponent))))
  (bind _output (`|GetArrayItem` (`self.Static mesh`) (- (`KismetStringLibrary.Conv_StringToInt` _returnvalue) 1)))
  ;[1 1 1] Get tags and checks them when 'Add Code' is run
  (cast `/Game/FirstPerson/Blueprints/BP_FirstPersonCharacter` OtherActor)
  (`KismetSystemLibrary.PrintString` "Triggered!")
  (`self.AddCode` _returnvalue)
  (`PrimitiveComponent.SetMaterial` _output 0 (select `bool` (== (`PrimitiveComponent.GetMaterial` _output 0) (`self.Color1`)) :`false` (`self.Color1`) :`true` (`self.Color2`)))
  (`KismetSystemLibrary.PrintString` _returnvalue true true (struct :`R` 0.970833 :`G` 0.941667 :`B` 1.0 :`A` 1.0) 5.0)
  (return))

(fn `UserConstructionScript`
  ;[1 1 1] Generate and space pressure plates basd on no. characters in correct code. Change mesh and material in "Add Static Mesh Component"
  (for _index (range (`KismetStringLibrary.Len` (`self.CorrectCode`)))
    (bind _returnvalue (`AddComponent|NODE_AddSM_PressurePlate-1` :`RelativeTransform` (`KismetMathLibrary.MakeTransform` (`KismetMathLibrary.MakeVector` (* _index (`self.Spacing`))))))
    (`KismetArrayLibrary.Array_Add` (`/Game/Assets/Environment/Interactables/PressurePlates/SM_PressurePlateA.Static mesh` _returnvalue) _returnvalue)
    ;[1 1 1] Set Tags and Create Event on Component Overlap
    (set `ActorComponent.ComponentTags` (`|MakeArray` (`KismetStringLibrary.Conv_StringToName` (`KismetStringLibrary.GetSubstring` (`self.CodeAssign`) _index))) _returnvalue)
    (add `PrimitiveComponent.OnComponentBeginOverlap` _returnvalue (`|CreateDelegate` :!event `EventTriggerFunction`))))